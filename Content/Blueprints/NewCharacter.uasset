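; NewCharacter is a player-controlled 2D flipbook character that moves and animates in four directions.
; The UpOrDown and LeftOrRight axes feed movement input along world Z and X.
; Each tick, SetMyFlipbook stores the last input direction, with vertical taking priority over horizontal.
; It then picks that direction's move flipbook while velocity is non-zero, or its idle flipbook otherwise.
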(event `self.ReceiveTick`
  (params (DeltaSeconds :type "Float (single-precision)"))
  (`self.SetMyFlipbook`))

(event `InputAxis|UpOrDown`
  (params (AxisValue :type "Float (single-precision)"))
  (`self.AddMovementInput` (0.0 0.0 1.0) AxisValue))

(event `InputAxis|LeftOrRight`
  (params (AxisValue :type "Float (single-precision)"))
  (`self.AddMovementInput` (1.0 0.0 0.0) AxisValue))

(fn `SetMyFlipbook`
  (bind _lastmovedirection (`self.LastMoveDirection`))
  (if (or (!= (`self.GetInputAxisValue`) 0.0) (!= (`self.GetInputAxisValue`) 0.0))
    (set `self.LastMoveDirection` (select `bool` (> (`self.GetInputAxisValue`) 0.0) :`false` (select `bool` (< (`self.GetInputAxisValue`) 0.0) :`false` (select `bool` (> (`self.GetInputAxisValue`) 0.0) :`false` "NewEnumerator2" :`true` "NewEnumerator3" :!type "/Game/Character/MoveDirection Enum") :`true` "NewEnumerator1") :`true` "NewEnumerator0")))
  (`PaperFlipbookComponent.SetFlipbook` (`self.Sprite`) (select `bool` (> (`KismetMathLibrary.VSize` (`self.GetVelocity`)) 0.0) :`false` (select `/Game/Character/MoveDirection` _lastmovedirection :`NewEnumerator0` "/Game/Character/IdleUp.IdleUp" :`NewEnumerator1` "/Game/Character/IdleDown.IdleDown" :`NewEnumerator2` "/Game/Character/IdleLeft.IdleLeft" :`NewEnumerator3` "/Game/Character/IdleRight.IdleRight" :!type "PaperFlipbook Object Reference") :`true` (select `/Game/Character/MoveDirection` _lastmovedirection :`NewEnumerator0` "/Game/Character/MoveUp.MoveUp" :`NewEnumerator1` "/Game/Character/MoveDown.MoveDown" :`NewEnumerator2` "/Game/Character/MoveLeft.MoveLeft" :`NewEnumerator3` "/Game/Character/MoveRight.MoveRight" :!type "PaperFlipbook Object Reference"))))

(fn `UserConstructionScript`)